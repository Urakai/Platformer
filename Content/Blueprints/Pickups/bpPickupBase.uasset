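; Base pickup actor that homes in on the player and is collected on contact.
; Entering the outer collision stores the player, after which Tick points the projectile movement velocity straight at them at IncreaseSpeed, as the lerp alpha is 1.
; Touching the inner collision reports the pickup to bpGameController, the game mode cached on BeginPlay, then destroys the actor.
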(event `self.ReceiveBeginPlay`
  (bind _asbp_game_controller (cast `/Game/Blueprints/Misc/bpGameController` (`GameplayStatics.GetGameMode`)))
  (set `self.GameController` _asbp_game_controller))

(event `self.InnerCollision.OnComponentBeginOverlap`
  (params (OverlappedComponent :type "PrimitiveComponent Object Reference") (OtherActor :type "Actor Object Reference") (OtherComp :type "PrimitiveComponent Object Reference") (OtherBodyIndex :type Integer) (bFromSweep :type Boolean) (SweepResult :type "HitResult Structure (by ref)"))
  (cast `/Game/Blueprints/Misc/bpPlayer` OtherActor)
  (`/Game/Blueprints/Misc/bpGameController.OnPickUp` (`self.GameController`) self)
  (`self.K2_DestroyActor`))

(event `self.ReceiveTick`
  (params (DeltaSeconds :type "Float (single-precision)"))
  (bind _projectilemovement (`self.ProjectileMovement`))
  (`/Engine/EditorBlueprintResources/StandardMacros.IsValid` (`self.BpPlayer`)
    (:`Is Valid`
      (set `MovementComponent.Velocity` (`KismetMathLibrary.VLerp` (`MovementComponent.Velocity` _projectilemovement) (* (`KismetMathLibrary.Normal` (- (`self.K2_GetActorLocation` (`self.BpPlayer`)) (`self.K2_GetActorLocation`))) (`self.IncreaseSpeed`)) 1.0) _projectilemovement))))

(event `self.OuterCollision.OnComponentBeginOverlap`
  (params (OverlappedComponent :type "PrimitiveComponent Object Reference") (OtherActor :type "Actor Object Reference") (OtherComp :type "PrimitiveComponent Object Reference") (OtherBodyIndex :type Integer) (bFromSweep :type Boolean) (SweepResult :type "HitResult Structure (by ref)"))
  (bind _asbp_player (cast `/Game/Blueprints/Misc/bpPlayer` OtherActor))
  (`/Engine/EditorBlueprintResources/StandardMacros.IsValid` (`self.BpPlayer`)
    (:`Is Not Valid`
      (set `self.BpPlayer` _asbp_player))))

(fn `UserConstructionScript`)
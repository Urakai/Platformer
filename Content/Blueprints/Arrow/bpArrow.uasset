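; Arrow actor that damages the player on hit or wobbles in place when it hits anything else.
; A hit on bpPlayer applies damage and destroys the arrow immediately.
; Any other hit plays the Wobble timeline, whose updates rotate the Scene component, disable collision and start a short delay before the arrow destroys itself.
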(event `self.ReceiveHit`
  (params (MyComp :type "PrimitiveComponent Object Reference") (Other :type "Actor Object Reference") (OtherComp :type "PrimitiveComponent Object Reference") (bSelfMoved :type Boolean) (HitLocation :type "Vector Structure") (HitNormal :type "Vector Structure") (NormalImpulse :type "Vector Structure") (Hit :type "HitResult Structure (by ref)"))
  (bind _asbp_player (cast `/Game/Blueprints/Misc/bpPlayer` Other)
    (:`then`
      (bind _output_get (set `self.CharacterBP` _asbp_player))
      (`GameplayStatics.ApplyDamage` _output_get 1.0)
      (`self.K2_DestroyActor`))
    (:`CastFailed`
      (bind (_direction _wobble) (`Timeline|Wobble`)
        (:`Update`
          (`SceneComponent.K2_SetRelativeRotation` (`self.Scene`) (`KismetMathLibrary.RLerp` (struct) (struct :`Pitch` 10.0) _wobble) false false)
          (`PrimitiveComponent.SetCollisionEnabled` (`self.Collision`) "NoCollision")
          (`KismetSystemLibrary.Delay` 3.0)
          (`self.K2_DestroyActor`))))))

(fn `UserConstructionScript`)
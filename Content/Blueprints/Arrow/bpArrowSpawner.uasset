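; Arrow spawner actor that fires arrows repeatedly while moving vertically.
; On BeginPlay it starts a looping one-second timer that calls Fire, which spawns a BpArrow at the SpawnPoint transform.
; It also plays the Movement timeline, lerping its location from the start position along Z, with Speed as the offset distance and the timeline value scaled by Move as alpha.
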(event `self.ReceiveBeginPlay`
  (bind (_start_pos_x _start_pos_y _start_pos_z) (`KismetMathLibrary.BreakVector` (`self.Start Pos`)))
  (set `self.Start Pos` (`self.K2_GetActorLocation`))
  (`KismetSystemLibrary.K2_SetTimer` null "Fire" 1.0 true)
  (bind (_direction _move) (`Timeline|Movement` :`NewTime` 0.0 :!via `PlayFromStart`)
    (:`Update`
      (`self.K2_SetActorLocation` (`KismetMathLibrary.VLerp` (`self.Start Pos`) (`KismetMathLibrary.MakeVector` _start_pos_x _start_pos_y (+ _start_pos_z (`self.Speed`))) (* _move (`self.Move`)))))))

(event `Fire`
  (`|SpawnActorFromClass` "/Game/Blueprints/Arrow/bpArrow.bpArrow_C" (`SceneComponent.K2_GetComponentToWorld` (`self.SpawnPoint`)) "Undefined" "OverrideRootScale"))

(fn `UserConstructionScript`)
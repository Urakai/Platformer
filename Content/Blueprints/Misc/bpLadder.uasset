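; A climbable ladder Blueprint that lets bpPlayer climb while inside its Box trigger.
; The construction script stacks collision-free Paper2D rung sprites at a fixed spacing over the LadderTop-to-LadderBottom height, then scales and raises the Box to match.
; Box overlap toggles the player's CanClimb; leaving also calls ClimbingEnd and restores StaticMesh collision.
; An AllowDown event re-runs the begin-overlap logic to re-enable climbing.
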(event `self.Box.OnComponentBeginOverlap`
  (params (OverlappedComponent :type "PrimitiveComponent Object Reference") (OtherActor :type "Actor Object Reference") (OtherComp :type "PrimitiveComponent Object Reference") (OtherBodyIndex :type Integer) (bFromSweep :type Boolean) (SweepResult :type "HitResult Structure (by ref)"))
  (bind _asbp_player (cast `/Game/Blueprints/Misc/bpPlayer` OtherActor :!label _label))
  (set `/Game/Blueprints/Misc/bpPlayer.bCanClimb` true _asbp_player))

(event `self.Box.OnComponentEndOverlap`
  (params (OverlappedComponent :type "PrimitiveComponent Object Reference") (OtherActor :type "Actor Object Reference") (OtherComp :type "PrimitiveComponent Object Reference") (OtherBodyIndex :type Integer))
  (bind _asbp_player (cast `/Game/Blueprints/Misc/bpPlayer` OtherActor))
  (set `/Game/Blueprints/Misc/bpPlayer.bCanClimb` false _asbp_player)
  (`/Game/Blueprints/Misc/bpPlayer.ClimbingEnd` _asbp_player)
  (`PrimitiveComponent.SetCollisionEnabled` (`self.StaticMesh`) "QueryAndPhysics"))

(event `AllowDown`
  (goto _label))

(fn `UserConstructionScript`
  (bind _box (`self.Box`))
  (bind _rungoffset (`self.RungOffset`))
  (bind (_returnvalue_x _returnvalue_y _returnvalue_z) (`KismetMathLibrary.BreakVector` (- (`self.LadderTop`) (`self.LadderBottom`))))
  (bind _returnvalue (/ _returnvalue_z 2.0))
  (`|ExecutionSequence`
    (:`then_0`
      ;[1 1 1] Ladder Construction
      (for _index (range (+ (`KismetMathLibrary.FTrunc` (/ _returnvalue_z _rungoffset)) 1))
        (bind _returnvalue_2 (`AddComponent|NODE_AddPaperSpriteComponent-0` :`RelativeTransform` (`KismetMathLibrary.MakeTransform` (`KismetMathLibrary.MakeVector` 0.0 0.0 (* _index _rungoffset)) (struct) (1.0 1.0 0.1))))
        (`PaperSpriteComponent.SetSprite` _returnvalue_2 (`self.LadderSprite`))
        (`PrimitiveComponent.SetCollisionEnabled` _returnvalue_2 "NoCollision")
        (`PrimitiveComponent.SetCollisionEnabled` _returnvalue_2 "NoCollision"))
      (`SceneComponent.SetRelativeScale3D` _box (`KismetMathLibrary.MakeVector` 1.0 1.0 _returnvalue))
      (`SceneComponent.K2_AddRelativeLocation` _box (`KismetMathLibrary.MakeVector` 0.0 0.0 _returnvalue) false false))))
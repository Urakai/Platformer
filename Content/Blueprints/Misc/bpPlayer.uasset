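; Player character for a 2D side-scroller with jumping, wall jumps, dashing, ladder climbing, projectile firing and health.
; Input events drive movement through launches and Flying mode, using line traces to find walls and ladders.
; Tick flips the sprite and picks flipbooks via a priority-based state function, while timelines add squash-and-stretch to jumps and landings.
; Zero health destroys the actor; mushroom growth and ring dropping exist, but their damage branch is disconnected.
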(event `self.ReceiveBeginPlay`
  ;[1 1 1] Begin Play
  (bind _asbp_game_controller (cast `/Game/Blueprints/Misc/bpGameController` (`GameplayStatics.GetGameMode`)))
  (set `self.bpGameController` _asbp_game_controller))

(event `self.ReceiveTick`
  (params (DeltaSeconds :type "Float (single-precision)"))
  (bind _sprite (`self.Sprite`))
  ;[1 0.5594 0.6093] Update/Rotate sprite
  (`self.Update Animation`)
  (`/Engine/EditorBlueprintResources/StandardMacros.CompareFloat` (.x (`MovementComponent.Velocity` (`self.CharacterMovement`)))
    (:`>`
      (`SceneComponent.K2_SetRelativeRotation` :`self` _sprite))
    (:`<`
      (`SceneComponent.K2_SetRelativeRotation` _sprite (struct :`Yaw` 180.0) false false))))

(event `InputAxis|Right`
  (params (AxisValue :type "Float (single-precision)"))
  ;[0.3102 0.2825 1] Movement
  (if (`self.bCanMoveRight`)
    (`self.AddMovementInput` (1.0 0.0 0.0) AxisValue)))

(event `self.OnLanded`
  (params (Hit :type "HitResult Structure (by ref)"))
  ;[1 1 1] Landed
  (`self.LandFX`))

(event `InputAction|Dash`
  (params (Key :type "Key Structure" :default "AnyKey"))
  (bind _returnvalue (`self.GetVelocity`))
  ;[1 1 1] Dash
  (:`Pressed`
    (if (!= _returnvalue (0.0 0.0 0.0))
      (if (`NavMovementComponent.IsFalling` (`self.CharacterMovement`))
        (`self.LaunchCharacter` (* (+ _returnvalue (0.0 0.0 0.0)) (1.5 1.5 1.5)) true true)
        (else
          (`self.LaunchCharacter` (* (+ _returnvalue (0.0 0.0 1.0)) (1.5 1.5 250.0))))))))

(event `InputAction|Jump`
  (params (Key :type "Key Structure" :default "AnyKey"))
  ;[0.3065 1 0.6217] Jumping
  (:`Pressed`
    (set `self.bCanMoveRight` true)
    (if (`NavMovementComponent.IsFalling` (`self.CharacterMovement`))
      (`self.WallJump`)
      (else
        (`self.Jump`)
        (`self.JumpFX`))))
  (:`Released`
    (`self.StopJumping`)))

(event `WallJump`
  (bind _returnvalue (`self.GetActorForwardVector`))
  (bind _returnvalue_x (`KismetMathLibrary.BreakVector` (`self.K2_GetActorLocation`)))
  ;[1 1 1] Wall Jump
  (bind (_outhit _returnvalue_2) (`KismetSystemLibrary.LineTraceSingle` (- (`self.K2_GetActorLocation`) (* _returnvalue (+ (`CapsuleComponent.GetScaledCapsuleRadius` (`self.CapsuleComponent`)) 15.0))) (+ (`self.K2_GetActorLocation`) (* _returnvalue (+ (`CapsuleComponent.GetScaledCapsuleRadius` (`self.CapsuleComponent`)) 15.0))) "TraceTypeQuery1" true))
  (if _returnvalue_2
    (`self.LaunchCharacter` (`KismetMathLibrary.MakeVector` (* (`KismetMathLibrary.SignOfFloat` (- _returnvalue_x (.x (`.Location` (`GameplayStatics.BreakHitResult` _outhit))))) 450.0) 0.0 (`CharacterMovementComponent.JumpZVelocity` (`self.CharacterMovement`))) true true)
    (`self.JumpFX`)
    (elif (< (`self.JumpCurrentCount`) (`self.JumpMaxCount`))
      (`self.Jump`)
      (`self.JumpFX`))))

(event `JumpFX`
  ;[1 1 1] JumpF FX
  (`GameplayStatics.SpawnEmitterAtLocation` "/Game/Art/Particles/p_dust.p_dust" (`SceneComponent.K2_GetComponentLocation` (`self.DustBox`)))
  (bind (_direction _squash) (`Timeline|TJump` :!via `PlayFromStart`)
    (:`Update`
      (`self.SetActorScale3D` (`KismetMathLibrary.VLerp` (`self.CurrentScale`) (0.5 1.0 2.0) _squash)))))

(event `LandFX`
  ;[1 1 1] JumpF FX
  (`GameplayStatics.SpawnEmitterAtLocation` "/Game/Art/Particles/p_dust.p_dust" (`SceneComponent.K2_GetComponentLocation` (`self.DustBox`)))
  (bind (_direction _squash) (`Timeline|TLand` :!via `PlayFromStart`)
    (:`Update`
      (`self.SetActorScale3D` (`KismetMathLibrary.VLerp` (`self.CurrentScale`) (2.0 1.0 0.75) _squash)))))

(event `Update Animation`
  (bind _returnvalue (`NavMovementComponent.IsFalling` (`self.CharacterMovement`)))
  ;[1 1 1] Control Animation
  (set `self.bIsMoving` (> (`KismetMathLibrary.VSize` (`self.GetVelocity`)) 0.0))
  (bind _output_fp (`self.AnimationStateMachine` (`self.bIsMoving`) _returnvalue _returnvalue (`self.bIsAttacking`) (`self.bIsClimbing`)))
  (`PaperFlipbookComponent.SetFlipbook` (`self.Sprite`) _output_fp))

(event `FireProjectile`
  ;[1 1 1] Attacking
  (`|SpawnActorFromClass` "/Game/Blueprints/Arrow/bpProjectile.bpProjectile_C" (`SceneComponent.K2_GetComponentToWorld` (`self.ProjectileSpawn`)) "AlwaysSpawn" "OverrideRootScale")
  (set `self.bIsAttacking` false))

(event `InputAction|Fire`
  (params (Key :type "Key Structure" :default "AnyKey"))
  ;[1 1 1] Attacking
  (:`Pressed`
    (set `self.bIsAttacking` true)
    (`self.FireProjectile`)))

(event `InputAxis|MoveUp`
  (params (AxisValue :type "Float (single-precision)"))
  ;[1 0.9744 0.04598] Climb Input
  (`self.DetectLater`)
  (if (`self.bCanClimb`)
    (if (`KismetMathLibrary.InRange_FloatFloat` AxisValue -0.1 0.1)
      ;;[1 0.02983 0] Climb - Anim Stop
      (`PaperFlipbookComponent.SetPlayRate` (`self.Sprite`) 0.0)
      (else
        ;;[0.0733 1 0] Climb - Anim Start
        (set `self.bIsClimbing` true)
        (set `self.bCanMoveRight` false)
        (`PaperFlipbookComponent.SetPlayRate` (`self.Sprite`) 1.0)
        ;;[0.5383 0.4202 1] Move Char Up/Down
        (`CharacterMovementComponent.SetMovementMode` (`self.CharacterMovement`) "MOVE_Flying" 0)
        (`self.AddMovementInput` (0.0 0.0 0.5) AxisValue)))))

(event `ClimbingEnd`
  ;[1 1 1] Climb End
  (`CharacterMovementComponent.SetMovementMode` (`self.CharacterMovement`) "MOVE_Walking" 0)
  (set `self.bIsClimbing` false)
  (set `self.bCanMoveRight` true)
  (`PaperFlipbookComponent.SetPlayRate` (`self.Sprite`) 1.0) ; Returns anim speed to normal
)

(event `DetectLater`
  (bind _returnvalue (`self.K2_GetActorLocation`))
  ;[1 1 1] Move Through Collision
  (bind _outhit (`KismetSystemLibrary.LineTraceSingle` :`Start` _returnvalue :`End` (`KismetMathLibrary.MakeVector` (.x _returnvalue) (.y _returnvalue) (+ (.z _returnvalue) (* (`self.GetInputAxisValue`) 20.0))) :`TraceChannel` "TraceTypeQuery1" :`DrawDebugType` "ForOneFrame"))
  (bind _asbp_ladder (cast `/Game/Blueprints/Misc/bpLadder` (`.HitActor` (`GameplayStatics.BreakHitResult` _outhit))))
  (`/Game/Blueprints/Misc/bpLadder.AllowDown` _asbp_ladder)
  (`PrimitiveComponent.SetCollisionEnabled` (`/Game/Blueprints/Misc/bpLadder.StaticMesh` _asbp_ladder) "NoCollision"))

(event `Scale Control`
  (params (bIsHealth :type Boolean))
  (if bIsHealth
    (if (not (`/Game/Blueprints/Misc/bpGameController.bHasMushroom` (`self.bpGameController`)))
      (bind (_direction _scale_lerp) (`Timeline|Scale`)
        (:`Update`
          (`self.SetActorScale3D` _scale_lerp)
          (set `self.CurrentScale` (`self.IncreasedScale`))
          (set `/Game/Blueprints/Misc/bpGameController.bHasMushroom` true (`self.bpGameController`)))))
    (else
      (bind _output_get (set `self.CurrentScale` (`self.StartScale`)))
      (`self.SetActorScale3D` _output_get)
      (set `/Game/Blueprints/Misc/bpGameController.bHasMushroom` false (`self.bpGameController`)))))

(event `self.ReceiveAnyDamage`
  (params (Damage :type "Float (single-precision)") (DamageType :type "DamageType Object Reference") (InstigatedBy :type "Controller Object Reference") (DamageCauser :type "Actor Object Reference"))
  ;[1 1 1] Damage
  (set `self.Health` (- (`self.Health`) Damage))
  (if (not (> (`self.Health`) 0.0))
    (`GameplayStatics.SpawnEmitterAtLocation` "/Game/Art/Particles/p_dust.p_dust" (`self.K2_GetActorLocation`))
    (`self.K2_DestroyActor`)))

(event `DropRing`
  ;[1 1 1] DropRing
  (for _ (range (`/Game/Blueprints/Misc/bpGameController.RingsCollected` (`self.bpGameController`)))
    (`|SpawnActorFromClass` "/Game/Blueprints/Pickups/bpPickupRing.bpPickupRing_C" (`self.GetTransform`) "Undefined" "OverrideRootScale" null true))
  (set `/Game/Blueprints/Misc/bpGameController.RingsCollected` 0 (`self.bpGameController`)))

(event `Heal`
  (params (HP :type "Float (double-precision)"))
  (bind _returnvalue (+ HP (`self.Health`)))
  ;[1 1 1] Heal
  (if (< _returnvalue (`self.MaxHealth`))
    (set `self.Health` _returnvalue)
    (else
      (set `self.Health` (`self.MaxHealth`)))))

(fn `AnimationStateMachine`
  (params (bisMoving :type Boolean) (bisFalling :type Boolean) (bisDashing :type Boolean) (bisAttacking :type Boolean) (bisClimbing :type Boolean))
  (returns (output_fp :type "PaperFlipbook Object Reference"))
  (locals (AnimationState :type "/Game/Data/AnimationState Enum" :default "NewEnumerator0"))
  (if bisClimbing
    (set `local.AnimationState` "NewEnumerator5")
    (elif bisDashing
      (set `local.AnimationState` "NewEnumerator4")
      (elif bisAttacking
        (set `local.AnimationState` "NewEnumerator3")
        (elif bisFalling
          (set `local.AnimationState` "NewEnumerator2")
          (elif bisMoving
            (set `local.AnimationState` "NewEnumerator1")
            (else
              (set `local.AnimationState` "NewEnumerator0")))))))
  (return (select `/Game/Data/AnimationState` (`local.AnimationState`) :`NewEnumerator0` (`self.IdleFB`) :`NewEnumerator1` (`self.RunningFB`) :`NewEnumerator2` (`self.JumpingFB`) :`NewEnumerator4` (`self.DashingFB`) :`NewEnumerator3` (`self.DashingFB`) :`NewEnumerator5` (`self.ClimbingFB`))))

(fn `UserConstructionScript`
  (set `CharacterMovementComponent.JumpZVelocity` 400.0 (`self.CharacterMovement`))
  (set `self.JumpMaxHoldTime` 0.3)
  ;[1 1 1] actors starting scale
  (bind _output_get (set `self.StartScale` (`self.GetActorScale3D`)))
  (set `self.CurrentScale` _output_get)
  ;[1 1 1] Initialize Health
  (set `self.Health` (`self.MaxHealth`)))
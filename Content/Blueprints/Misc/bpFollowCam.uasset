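; Follow camera actor that tracks the first player's pawn at a world offset with a fixed rotation.
; Each Tick, while the pawn is valid, it sets its transform with TInterpTo toward the pawn's location plus WolrdOffset.
; The interpolation start takes X from the pawn and Y and Z from the actor, plus the same offset, so X stays locked to the pawn.
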(event `self.ReceiveTick`
  (params (DeltaSeconds :type "Float (single-precision)"))
  (bind _returnvalue (`GameplayStatics.GetPlayerPawn` 0))
  (bind _returnvalue_2 (`self.GetTransform` _returnvalue))
  (`/Engine/EditorBlueprintResources/StandardMacros.IsValid` _returnvalue
    (:`Is Valid`
      (`self.K2_SetActorTransform` (`KismetMathLibrary.TInterpTo` (`KismetMathLibrary.MakeTransform` (+ (`KismetMathLibrary.MakeVector` (.x (.location _returnvalue_2)) (.y (.location (`self.GetTransform`))) (.z (.location (`self.GetTransform`)))) (`self.WolrdOffset`)) (struct :`Yaw` -90.0)) (`KismetMathLibrary.MakeTransform` (+ (.location _returnvalue_2) (`self.WolrdOffset`)) (struct :`Yaw` -90.0)) DeltaSeconds)))))

(fn `UserConstructionScript`)
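; Paper2D patrolling enemy that damages and knocks back the player on contact.
; The construction script feeds PointA and PointB to an InterpToMovement component as relative control points, and a FlipFlop turns the flipbook around each time movement reverses.
; When the Box overlaps a bpPlayer, it applies fixed damage and launches the player upward and horizontally along X based on the sweep normal.
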(event `self.InterpToMovement.OnInterpToReverse`
  (params (ImpactResult :type "HitResult Structure (by ref)") (Time :type "Float (single-precision)"))
  (bind _paperflipbook (`self.PaperFlipbook`))
  (`/Engine/EditorBlueprintResources/StandardMacros.FlipFlop`
    (:`A`
      (`SceneComponent.K2_SetRelativeRotation` _paperflipbook (struct :`Yaw` 180.0) false false))
    (:`B`
      (`SceneComponent.K2_SetRelativeRotation` _paperflipbook (struct) false false))))

(event `self.Box.OnComponentBeginOverlap`
  (params (OverlappedComponent :type "PrimitiveComponent Object Reference") (OtherActor :type "Actor Object Reference") (OtherComp :type "PrimitiveComponent Object Reference") (OtherBodyIndex :type Integer) (bFromSweep :type Boolean) (SweepResult :type "HitResult Structure (by ref)"))
  (bind _asbp_player (cast `/Game/Blueprints/Misc/bpPlayer` OtherActor))
  (`GameplayStatics.ApplyDamage` _asbp_player 10.0 null null "/Script/Engine.DamageType")
  (`Character.LaunchCharacter` _asbp_player (`KismetMathLibrary.MakeVector` (* (.x (`.Normal` (`GameplayStatics.BreakHitResult` SweepResult))) -400.0) 0.0 200.0) true true))

(fn `UserConstructionScript`
  (set `InterpToMovementComponent.ControlPoints` (`|MakeArray` (make `InterpControlPoint` (`self.Point A`)) (make `InterpControlPoint` (`self.Point B`))) (`self.InterpToMovement`)))
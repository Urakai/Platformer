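; Moving platform actor that shifts between its starting position and an offset from it.
; On BeginPlay it stores its location and plays the Movement timeline from the start.
; Each update lerps the actor toward the start plus the Speed vector using the timeline's Move track, so Speed acts as a travel offset rather than a velocity.
; Movement is applied without sweep, so it ignores blocking collisions along the path.
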(event `self.ReceiveBeginPlay`
  (bind (_start_pos_x _start_pos_y _start_pos_z) (`KismetMathLibrary.BreakVector` (`self.Start Pos`)))
  (bind (_speed_x _speed_y _speed_z) (`KismetMathLibrary.BreakVector` (`self.Speed`)))
  (set `self.Start Pos` (`self.K2_GetActorLocation`))
  (bind (_direction _move) (`Timeline|Movement` :!via `PlayFromStart`)
    (:`Update`
      (`self.K2_SetActorLocation` (`KismetMathLibrary.VLerp` (`self.Start Pos`) (`KismetMathLibrary.MakeVector` (+ _start_pos_x _speed_x) (+ _start_pos_y _speed_y) (+ _start_pos_z _speed_z)) _move)))))

(fn `UserConstructionScript`)
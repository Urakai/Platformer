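; Player controller that lets the player swap between two character pawns and tracks health on the controller, so it carries across swaps.
; The Swap input spawns the other of BP_Player1 or BP_Player2 at the current pawn's transform, possesses it and destroys the old pawn.
; UpdateHealth subtracts damage from Health, initialized to MaxHealth in the construction script, and at zero spawns a dust effect and destroys the controlled pawn.
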(event `InputAction|Swap`
  (params (Key :type "Key Structure" :default "AnyKey"))
  (:`Pressed`
    (bind _output_get (set `self.PreviousPawn` (`self.K2_GetPawn`)))
    (bind _asbp_player_1 (cast `/Game/Blueprints/Misc/BP_Player1` _output_get)
      (:`then`
        (bind _returnvalue (`|SpawnActorFromClass` "/Game/Blueprints/Misc/BP_Player2.BP_Player2_C" (`self.GetTransform` _asbp_player_1) "Undefined" "OverrideRootScale"))
        (`self.Possess` _returnvalue)
        (`self.K2_DestroyActor` (`self.PreviousPawn`)))
      (:`CastFailed`
        (bind _returnvalue_2 (`|SpawnActorFromClass` "/Game/Blueprints/Misc/BP_Player1.BP_Player1_C" (`self.GetTransform` (`self.PreviousPawn`)) "Undefined" "OverrideRootScale"))
        (`self.Possess` _returnvalue_2)
        (`self.K2_DestroyActor` (`self.PreviousPawn`))))))

(event `UpdateHealth`
  (params (Delta :type "Float (double-precision)"))
  (bind _returnvalue (`self.K2_GetPawn`))
  (set `self.Health` (- (`self.Health`) Delta))
  (if (not (> (`self.Health`) 0.0))
    (`GameplayStatics.SpawnEmitterAtLocation` "/Game/Art/Particles/p_dust.p_dust" (`self.K2_GetActorLocation` _returnvalue))
    (`self.K2_DestroyActor` _returnvalue)))

(fn `UserConstructionScript`
  ;[1 1 1] Initialize Health
  (set `self.Health` (`self.MaxHealth`)))
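; bpGameController is a game controller that creates the HUD and applies pickup effects to the player.
; On BeginPlay it adds a BpHUD widget to the viewport and caches player pawn 0 as a BP_PlayerBase reference.
; OnPickUp branches on the pickup's class by casting: mushrooms trigger the player's ScaleControl, rings increment a collected counter, and potions heal the player.
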(event `self.ReceiveBeginPlay`
  (bind _returnvalue (`|CreateWidget` "/Game/Blueprints/HUD/bpHUD.bpHUD_C"))
  (bind _output_get (set `self.HUDReference` _returnvalue))
  (`UserWidget.AddToViewport` _output_get 0)
  (bind _asbp_player_base (cast `/Game/Blueprints/Misc/BP_PlayerBase` (`GameplayStatics.GetPlayerPawn` 0)))
  (set `self.bpPlayer` _asbp_player_base))

(fn `OnPickUp`
  (params (PickUpType :type "/Game/Blueprints/Pickups/bpPickupBase Object Reference"))
  (cast `/Game/Blueprints/Pickups/bpPickupMushroom` PickUpType
    (:`then`
      (`/Game/Blueprints/Misc/BP_PlayerBase.Scale Control` (`self.bpPlayer`) true))
    (:`CastFailed`
      (cast `/Game/Blueprints/Pickups/bpPickupRing` PickUpType
        (:`then`
          (set `self.RingsCollected` (+ (`self.RingsCollected`) 1)))
        (:`CastFailed`
          (cast `/Game/Blueprints/Pickups/bpPickupPotion` PickUpType)
          (`/Game/Blueprints/Misc/BP_PlayerBase.Heal` (`self.bpPlayer`) 10.0))))))

(fn `UserConstructionScript`)